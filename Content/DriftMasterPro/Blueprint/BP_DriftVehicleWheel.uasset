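; Raycast wheel for the drift vehicle, simulating suspension and tire forces on the vehicle mesh.
; UpdateDelta loads tuning from WheelClass defaults, then each UpdatePhysics line-traces down, positions and spins the child wheel mesh, and applies spring-damper force.
; Throttle and lateral-slip forces, scaled by suspension load, are projected onto the ground plane.
; Computed ForceX and wheel angular velocity do not feed the applied forces or mesh spin.
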(event Custom|SubTickUpdatePhysics
  (params (SubTickDeltaTime :type Float%20%28double-precision%29)))

(event Custom|UpdateDelta
  (params (DebugMode :type Boolean) (VehicleMesh :type Primitive%20Component%20Object%20Reference))
  (Variables|Debug|SetDebugMode DebugMode)
  (Variables|Default|SetVehicleMesh VehicleMesh)
  (|GetDelta))

(event Custom|UpdatePhysics
  (params (Throttle :type Float%20%28double-precision%29) (DeltaTime :type Float%20%28double-precision%29))
  (Variables|Input|SetThrottle Throttle)
  (Variables|Delta|SetDeltaTime DeltaTime)
  (|Debug)
  (|WorldLocation/UpVector)
  (|RayCast)
  (|UpdateWheelMesh
    (:execute
      (if (Variables|Wheel|GetHit)
        (|GetSuspensionForce)
        (Physics|AddForce)
        (|GetLinearVelocityLocal)
        (|GetForceX
          (:execute
            (|WheelAcceleration
              (:execute
                (|GetThrottle/Steering)))))
        (else
          (|ResetValues))))))

(event EventBeginPlay
  (|GetMainDriftVehicle))

(fn SetWheelCoordinate
  (params (WheelCoordinate :type Drift%20Vehicle%20Coordinate%20Structure))
  (bind _output_get (Variables|Wheel|SetWheelCoordinate WheelCoordinate))
  (return _output_get))

(fn GetWheelCoordinate
  (return (Variables|Wheel|GetWheelCoordinate)))