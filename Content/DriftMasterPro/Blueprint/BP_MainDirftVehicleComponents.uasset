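; Vehicle controller component for a drift car that drives its wheel components and the physics-simulated static mesh root of its owner.
; On BeginPlay it caches the mesh and BP_DriftVehicleWheel components and hands the mesh to each wheel.
; Throttle and steering inputs are interpolated with rise/fall rates.
; Tick feeds throttle to wheel physics, yaws steering wheels using a speed curve and left/right Ackermann scaling, and updates forward km/h.
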(event `self.ReceiveBeginPlay`
  (bind _returnvalue (`self.GetOwner`))
  (`|ExecutionSequence`
    (:`then_0`
      (bind _asstatic_mesh_component (cast `StaticMeshComponent` (`Actor.RootComponent` _returnvalue))
        (:`then`
          (set `self.VehicleMesh` _asstatic_mesh_component))
        (:`CastFailed`
          (`KismetSystemLibrary.PrintString` "Not VehicleMesh!!!" true false (struct :`R` 1.0 :`B` 0.007 :`A` 1.0)))))
    (:`then_1`
      (set `self.Actor` _returnvalue)
      (bind _output_get (set `self.Wheel` (`Actor.K2_GetComponentsByClass` _returnvalue "/Game/DriftMasterPro/Blueprint/BP_DriftVehicleWheel.BP_DriftVehicleWheel_C")))
      (for _array_element _output_get
        (`/Game/DriftMasterPro/Blueprint/BP_DriftVehicleWheel.UpdateDelta` _array_element (`self.DebugMode`) (`self.VehicleMesh`)))
      (`PrimitiveComponent.SetSimulatePhysics` (`self.VehicleMesh`) true))))

(event `self.ReceiveTick`
  (params (DeltaSeconds :type "Float (single-precision)"))
  (bind _steeringindex (`self.SteeringIndex`))
  (bind _actor (`self.Actor`))
  (bind _returnvalue (> _steeringindex 0.0))
  (bind _output_get (set `self.DeltaTime` DeltaSeconds))
  (`/Game/DriftMasterPro/Blueprint/BP_DriftVehicleWheel.UpdatePhysics` (`self.Wheel`) (`self.ThrottleIndex`) _output_get)
  (for _array_element (`self.SteeringWheel`)
    (bind _returnvalue_2 (* (`.SteerAngle` (defaults `Object` (`/Game/DriftMasterPro/Blueprint/BP_DriftVehicleWheel.WheelClass` _array_element))) (* _steeringindex (`CurveFloat.GetFloatValue` (`self.SteeringCurve`) (`self.Km/h`)))))
    (bind _returnvalue_3 (* _returnvalue_2 (`self.AckermannAccuracy`)))
    (bind (_wheelcoordinate_f _wheelcoordinate_r) (break `/Game/DriftMasterPro/Blueprint/DriftVehicleCoordinate` (`/Game/DriftMasterPro/Blueprint/BP_DriftVehicleWheel.GetWheelCoordinate` _array_element)))
    (`SceneComponent.K2_SetRelativeRotation` _array_element (`KismetMathLibrary.MakeRotator` (.roll (`SceneComponent.RelativeRotation` _array_element)) (.pitch (`SceneComponent.RelativeRotation` _array_element)) (select `bool` _wheelcoordinate_r :`false` (select `bool` _returnvalue :`false` _returnvalue_2 :`true` _returnvalue_3 :!type "Float (single-precision)") :`true` (select `bool` _returnvalue :`false` _returnvalue_3 :`true` _returnvalue_2 :!type "Float (single-precision)"))) false false)
    (set `self.Km/h` (* (`KismetMathLibrary.Dot_VectorVector` (`Actor.GetVelocity` _actor) (`Actor.GetActorForwardVector` _actor)) 0.036))))

(fn `GetInputRate`
  (params (InputTarget :type "Float (double-precision)") (InputRate :type "/Game/DriftMasterPro/Blueprint/DriftInputRate Structure") (NowInpot :type "Float (double-precision)"))
  (returns (OutputeInput :type "Float (double-precision)"))
  (bind (_riserate _fallrate) (break `/Game/DriftMasterPro/Blueprint/DriftInputRate` InputRate))
  (return (`KismetMathLibrary.FInterpTo` NowInpot InputTarget (`self.DeltaTime`) (select `bool` (== NowInpot 0.0) :`false` _riserate :`true` _fallrate))))

(fn `Steering`
  (params (SteeringIndex :type "Float (double-precision)"))
  (bind _outputeinput (`self.GetInputRate` SteeringIndex (`self.SteeringInputRate`) (`self.SteeringIndex`)))
  (set `self.SteeringIndex` _outputeinput))

(fn `Throttle`
  (params (Throttle :type "Float (double-precision)"))
  (bind _outputeinput (`self.GetInputRate` Throttle (`self.ThrottleInputRate`) (`self.ThrottleIndex`)))
  (set `self.ThrottleIndex` _outputeinput))