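; Drift vehicle Blueprint that forwards Throttle and Steering axis input to its drift vehicle components object.
; The construction script finds every BP_DriftVehicleWheel component and derives its front/rear and left/right coordinate from relative location.
; It spawns and attaches each wheel's meshes, mirrored on Y for the negative-Y side and offset by suspension drop and wheel offsets.
; Steerable wheels are registered in the SteeringWheel list inside that mesh loop.
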(event `InputAxis|Throttle`
  (params (AxisValue :type "Float (single-precision)"))
  (`/Game/DriftMasterPro/Blueprint/BP_MainDirftVehicleComponents.Throttle` (`self.BP_MainDirftVehicleComponents`) AxisValue))

(event `InputAxis|Steering`
  (params (AxisValue :type "Float (single-precision)"))
  (`/Game/DriftMasterPro/Blueprint/BP_MainDirftVehicleComponents.Steering` (`self.BP_MainDirftVehicleComponents`) AxisValue))

(fn `UserConstructionScript`
  (locals (Wheel :type "/Game/DriftMasterPro/Blueprint/BP_DriftVehicleWheel Object Reference"))
  (bind _wheel (`local.Wheel`))
  (bind (_offset _shapewidth _steerangle _mass _affectd_by_handbrake _suspensionmaxraise _suspensionmaxdrop) (defaults `Object` (`/Game/DriftMasterPro/Blueprint/BP_DriftVehicleWheel.WheelClass` (`local.Wheel`))))
  (`KismetArrayLibrary.Array_Clear` (`/Game/DriftMasterPro/Blueprint/BP_MainDirftVehicleComponents.SteeringWheel` (`self.BP_MainDirftVehicleComponents`)))
  (for _array_element (`self.K2_GetComponentsByClass` "/Game/DriftMasterPro/Blueprint/BP_DriftVehicleWheel.BP_DriftVehicleWheel_C")
    (set `local.Wheel` _array_element)
    (bind (_relativelocation_x _relativelocation_y) (`KismetMathLibrary.BreakVector` (`SceneComponent.RelativeLocation` _array_element)))
    (bind _returnvalue (< _relativelocation_y 0.0))
    (`/Game/DriftMasterPro/Blueprint/BP_DriftVehicleWheel.SetWheelCoordinate` _array_element (make `/Game/DriftMasterPro/Blueprint/DriftVehicleCoordinate` (> _relativelocation_x 0.0) _returnvalue))
    (for _array_element_2 (`/Game/DriftMasterPro/Blueprint/BP_DriftVehicleWheel.Mesh` (`local.Wheel`))
      (bind _returnvalue_2 (`AddComponent|NODE_AddStaticMeshComponent-0` :`RelativeTransform` (`KismetMathLibrary.MakeTransform` (0.0 0.0 0.0) (struct) (`KismetMathLibrary.MakeVector` 1.0 (select `bool` _returnvalue :`false` 1.0 :`true` -1.0) 1.0))))
      (`StaticMeshComponent.SetStaticMesh` _returnvalue_2 _array_element_2)
      (`SceneComponent.K2_AttachToComponent` _returnvalue_2 (`local.Wheel`) "None" "KeepRelative" "KeepRelative" "KeepRelative" true)
      (`SceneComponent.K2_SetRelativeLocation` _returnvalue_2 (+ (`KismetMathLibrary.MakeVector` 0.0 0.0 (* _suspensionmaxdrop -1.0)) (`KismetMathLibrary.MakeVector` (.x _offset) (* (.y _offset) (select `bool` _returnvalue :`false` 1.0 :`true` -1.0)) (.z _offset)) (`KismetMathLibrary.MakeVector` (.x (`/Game/DriftMasterPro/Blueprint/BP_DriftVehicleWheel.Offset` (`local.Wheel`))) (* (.y (`/Game/DriftMasterPro/Blueprint/BP_DriftVehicleWheel.Offset` (`local.Wheel`))) (select `bool` _returnvalue :`false` 1.0 :`true` -1.0)) (.z (`/Game/DriftMasterPro/Blueprint/BP_DriftVehicleWheel.Offset` (`local.Wheel`))))) false false)
      (if (not (`/Game/DriftMasterPro/Blueprint/BP_DriftVehicleWheel.Disable Steering` _wheel))
        (`KismetArrayLibrary.Array_Add` (`/Game/DriftMasterPro/Blueprint/BP_MainDirftVehicleComponents.SteeringWheel` (`self.BP_MainDirftVehicleComponents`)) _wheel)))))